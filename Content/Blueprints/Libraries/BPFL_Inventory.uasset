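; Blueprint function library for a slot-based UMG inventory, offering setup, lookup, add and remove of items.
; InitializeInventory builds WB_Inventory on the HUD, creates its slots, then restores them from GI_Inventory's InventoryData or seeds that array.
; AddItem and RemoveItem find slots by item name, stack or clear quantities via UpdateQuantity, and refresh slot UI.
; Both scan loops return on the first slot, match or not, so later slots are never checked.
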(fn `AddItem`
  (params (ItemToAdd :type "/Game/Blueprints/Structs/ST_Item Structure") (QuantityToAdd :type Integer :default 1))
  (returns (SuccessfullyAdded :type Boolean))
  (locals (QuantityToAddRef :type Integer :default 1) (ItemToAddInfoRef :type "/Game/Blueprints/Structs/ST_Item Structure"))
  (set `local.ItemToAddInfoRef` ItemToAdd)
  (set `local.QuantityToAddRef` QuantityToAdd)
  (bind (_quantity _array_element _information _founditem) (`self.ScanForItem` (`.Name_17_84D617584D81D8513A3A4AB69E43B5DA` (break `/Game/Blueprints/Structs/ST_Item` (`local.ItemToAddInfoRef`)))))
  (if _founditem
    (`self.UpdateQuantity` _array_element (`local.QuantityToAddRef`))
    (return true)
    (else
      (bind (_foundemptyslot _slot) (`self.ScanForEmptySlot` null))
      (if _foundemptyslot
        (bind _output_get (set `/Game/Blueprints/Hero/UI/Inventory/WB_Inventory_Slot.Information` (`local.ItemToAddInfoRef`) _slot))
        (`|VariableSetRef` (`.Quantity_25_CB32A13742F8037488A8D990BE188642` (break `/Game/Blueprints/Structs/ST_Item` _output_get)) (`local.QuantityToAddRef`))
        (`/Game/Blueprints/Hero/UI/Inventory/WB_Inventory_Slot.UpdateUI` _slot)
        (return true)
        (else
          (return false))))))

(fn `GetHUD`
  (returns (HUDRef :type "/Game/Blueprints/Hero/UI/HUD/BP_HUD Object Reference"))
  (bind _foundwidgets (`WidgetBlueprintLibrary.GetAllWidgetsOfClass` null "/Game/Blueprints/Hero/UI/HUD/BP_HUD.BP_HUD_C"))
  (return (`|GetArrayItem` _foundwidgets)))

(fn `GetInventoryGameInstance`
  (returns (GameInstance :type "/Game/Blueprints/GI_Inventory Object Reference"))
  (bind _asgi_inventory (cast `/Game/Blueprints/GI_Inventory` (`GameplayStatics.GetGameInstance` null)))
  (return _asgi_inventory))

(fn `GetInventoryReference`
  (returns (InventoryRef :type "/Game/Blueprints/Hero/UI/Inventory/WB_Inventory Object Reference"))
  (bind _foundwidgets (`WidgetBlueprintLibrary.GetAllWidgetsOfClass` null "/Game/Blueprints/Hero/UI/Inventory/WB_Inventory.WB_Inventory_C" false))
  (return (`|GetArrayItem` _foundwidgets)))

(fn `InitializeInventory`
  (params (NumberOfSlots :type Integer) (ScreenAnchors :type "Anchors Structure"))
  (locals (HUDRef :type "/Game/Blueprints/Hero/UI/HUD/BP_HUD Object Reference") (InventoryPanel :type "/Game/Blueprints/Hero/UI/Inventory/WB_Inventory Object Reference") (GIRef :type "/Game/Blueprints/GI_Inventory Object Reference") (NewSlot :type "/Game/Blueprints/Hero/UI/Inventory/WB_Inventory_Slot Object Reference"))
  ;[1 1 1] Get Reference to HUD Blueprint
  (set `local.HUDRef` (`self.GetHUD` null))
  ;[1 1 1] Create core inventory panel widget and store a reference
  (bind _returnvalue (`|CreateWidget` "/Game/Blueprints/Hero/UI/Inventory/WB_Inventory.WB_Inventory_C"))
  (set `local.InventoryPanel` _returnvalue)
  (bind _returnvalue_2 (`CanvasPanel.AddChildToCanvas` (`/Game/Blueprints/Hero/UI/HUD/BP_HUD.MainPanel` (`local.HUDRef`)) _returnvalue))
  (`CanvasPanelSlot.SetAutoSize` _returnvalue_2 true)
  (`CanvasPanelSlot.SetAnchors` _returnvalue_2 ScreenAnchors)
  (`CanvasPanelSlot.SetOffsets` _returnvalue_2 (make `Margin` 0.0))
  (set `local.GIRef` (`self.GetInventoryGameInstance` null))
  (for _index (range NumberOfSlots)
    (bind _returnvalue_3 (`|CreateWidget` "/Game/Blueprints/Hero/UI/Inventory/WB_Inventory_Slot.WB_Inventory_Slot_C"))
    (set `local.NewSlot` _returnvalue_3)
    (set `/Game/Blueprints/Hero/UI/Inventory/WB_Inventory_Slot.InventoryIndex` _index (`local.NewSlot`))
    (`KismetArrayLibrary.Array_Add` (`/Game/Blueprints/Hero/UI/Inventory/WB_Inventory.InventorySlots` (`local.InventoryPanel`)) (`local.NewSlot`))
    (`WrapBox.AddChildToWrapBox` (`/Game/Blueprints/Hero/UI/Inventory/WB_Inventory.SlotsPanel` (`local.InventoryPanel`)) (`local.NewSlot`)))
  (if (> (`KismetArrayLibrary.Array_Length` (`/Game/Blueprints/GI_Inventory.InventoryData` (`local.GIRef`))) 0)
    (for (_array_element _array_index) (`/Game/Blueprints/Hero/UI/Inventory/WB_Inventory.InventorySlots` (`local.InventoryPanel`))
      (set `/Game/Blueprints/Hero/UI/Inventory/WB_Inventory_Slot.Information` (`|GetArrayItem` (`/Game/Blueprints/GI_Inventory.InventoryData` (`local.GIRef`)) _array_index) _array_element))
    (else
      (for _ (`/Game/Blueprints/Hero/UI/Inventory/WB_Inventory.InventorySlots` (`local.InventoryPanel`))
        (`KismetArrayLibrary.Array_Add` (`/Game/Blueprints/GI_Inventory.InventoryData` (`local.GIRef`)))))))

(fn `RemoveItem`
  (params (ItemToRemove :type "/Game/Blueprints/Structs/ST_Item Structure") (QuantityToRemove :type Integer :default 1))
  (returns (SuccessfullyRemoved :type Boolean))
  (bind (_quantity _array_element _information _founditem) (`self.ScanForItem` (`.Name_17_84D617584D81D8513A3A4AB69E43B5DA` (break `/Game/Blueprints/Structs/ST_Item` ItemToRemove))))
  (if _founditem
    (`self.UpdateQuantity` _array_element (* QuantityToRemove -1))
    (return true)
    (else
      (return false))))

(fn `ScanForEmptySlot`
  (returns (FoundEmptySlot :type Boolean) (Slot :type "/Game/Blueprints/Hero/UI/Inventory/WB_Inventory_Slot Object Reference"))
  (for _array_element (`/Game/Blueprints/Hero/UI/Inventory/WB_Inventory.InventorySlots` (`self.GetInventoryReference` null))
    (if (== (`.Name_17_84D617584D81D8513A3A4AB69E43B5DA` (break `/Game/Blueprints/Structs/ST_Item` (`/Game/Blueprints/Hero/UI/Inventory/WB_Inventory_Slot.Information` _array_element))) "None")
      (return true _array_element)
      (else
        (return false null))))
  (return true (`|GetArrayItem` (`/Game/Blueprints/Hero/UI/Inventory/WB_Inventory.InventorySlots` (`self.GetInventoryReference` null)))))

(fn `ScanForItem`
  (params (ItemToCheckFor :type Name))
  (returns (Quantity :type Integer) (`Array Element` :type "/Game/Blueprints/Hero/UI/Inventory/WB_Inventory_Slot Object Reference") (Information :type "/Game/Blueprints/Structs/ST_Item Structure") (FoundItem :type Boolean))
  (for _array_element (`/Game/Blueprints/Hero/UI/Inventory/WB_Inventory.InventorySlots` (`self.GetInventoryReference` null))
    (bind _information (`/Game/Blueprints/Hero/UI/Inventory/WB_Inventory_Slot.Information` _array_element))
    (bind (_name _type _icon _sprite _description _rarity _quantity) (break `/Game/Blueprints/Structs/ST_Item` _information))
    (if (== _name ItemToCheckFor)
      (return _quantity _array_element _information true)
      (else
        (return 0 null (struct) false))))
  (return 0 null (struct) false))

(fn `UpdateQuantity`
  (params (SlotToUpdate :type "/Game/Blueprints/Hero/UI/Inventory/WB_Inventory_Slot Object Reference") (QuantityToAdd :type Integer))
  (locals (Slot :type "/Game/Blueprints/Hero/UI/Inventory/WB_Inventory_Slot Object Reference") (FinalQuantity :type Integer :default 0))
  (bind _output_get (set `local.Slot` SlotToUpdate))
  (bind _output_get_2 (set `local.FinalQuantity` (+ (`.Quantity_25_CB32A13742F8037488A8D990BE188642` (break `/Game/Blueprints/Structs/ST_Item` (`/Game/Blueprints/Hero/UI/Inventory/WB_Inventory_Slot.Information` _output_get))) QuantityToAdd)))
  (if (<= _output_get_2 0)
    (set `/Game/Blueprints/Hero/UI/Inventory/WB_Inventory_Slot.Information` (struct) (`local.Slot`))
    (`/Game/Blueprints/Hero/UI/Inventory/WB_Inventory_Slot.UpdateUI` (`local.Slot`))
    (else
      (`|VariableSetRef` (`.Quantity_25_CB32A13742F8037488A8D990BE188642` (break `/Game/Blueprints/Structs/ST_Item` (`/Game/Blueprints/Hero/UI/Inventory/WB_Inventory_Slot.Information` (`local.Slot`)))) (`local.FinalQuantity`))
      (`/Game/Blueprints/Hero/UI/Inventory/WB_Inventory_Slot.UpdateUI` (`local.Slot`)))))