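; BP_Trap is an interactable prop that can damage the hero once and then destroy itself.
; An overlap with its Box component casts the other actor to BP_Hero and stores it as HeroRef, without dealing damage.
; The separate InflictDamage event, which nothing in this graph calls, subtracts a fixed amount directly from that hero's Health and destroys the trap.
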(event `self.InflictDamage`
  (set `/Game/Blueprints/Hero/BP_Hero.Health` (- (`/Game/Blueprints/Hero/BP_Hero.Health` (`self.HeroRef`)) 10.0) (`self.HeroRef`))
  (`self.K2_DestroyActor` self))

(event `self.Box.OnComponentBeginOverlap`
  (params (OverlappedComponent :type "PrimitiveComponent Object Reference") (OtherActor :type "Actor Object Reference") (OtherComp :type "PrimitiveComponent Object Reference") (OtherBodyIndex :type Integer) (bFromSweep :type Boolean) (SweepResult :type "HitResult Structure (by ref)"))
  (bind _asbp_hero (cast `/Game/Blueprints/Hero/BP_Hero` OtherActor))
  (if true
    (set `self.HeroRef` _asbp_hero)))

(fn `UserConstructionScript`)