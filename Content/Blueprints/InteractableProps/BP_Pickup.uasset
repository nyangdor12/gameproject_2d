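; BP_Pickup is an interactable item pickup that the hero collects into an inventory.
; The construction script loads item information from a data table row and applies its sprite, and BeginPlay writes "[E]" plus the item name on a widget nameplate.
; Hero overlap shows the nameplate and caches the hero, while end overlap hides it.
; Interact calls AddItem, and on success passes the item to the hero's BPC_Inventory and destroys the pickup.
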(event `self.ReceiveBeginPlay`
  (bind _aswb_pickup_namplate (cast `/Game/Blueprints/InteractableProps/WB_Pickup_Namplate` (`WidgetComponent.GetUserWidgetObject` (`self.NamePlate`))))
  (`TextBlock.SetText` (`/Game/Blueprints/InteractableProps/WB_Pickup_Namplate.NameText` _aswb_pickup_namplate) (`KismetTextLibrary.Conv_StringToText` (`KismetStringLibrary.Concat_StrStr` "[E]" (`KismetStringLibrary.Conv_NameToString` (`.Name_17_84D617584D81D8513A3A4AB69E43B5DA` (break `/Game/Blueprints/Structs/ST_Item` (`self.Information`))))))))

(event `self.InteractionCollider.OnComponentBeginOverlap`
  (params (OverlappedComponent :type "PrimitiveComponent Object Reference") (OtherActor :type "Actor Object Reference") (OtherComp :type "PrimitiveComponent Object Reference") (OtherBodyIndex :type Integer) (bFromSweep :type Boolean) (SweepResult :type "HitResult Structure (by ref)"))
  (if (`KismetMathLibrary.ClassIsChildOf` (`GameplayStatics.GetObjectClass` OtherActor) "/Game/Blueprints/Hero/BP_Hero.BP_Hero_C")
    (`SceneComponent.SetVisibility` (`self.NamePlate`) true false)
    (set `self.HeroRef` OtherActor)))

(event `self.InteractionCollider.OnComponentEndOverlap`
  (params (OverlappedComponent :type "PrimitiveComponent Object Reference") (OtherActor :type "Actor Object Reference") (OtherComp :type "PrimitiveComponent Object Reference") (OtherBodyIndex :type Integer))
  (if (`KismetMathLibrary.ClassIsChildOf` (`GameplayStatics.GetObjectClass` null) "/Game/Blueprints/Hero/BP_Hero.BP_Hero_C")
    (`SceneComponent.SetVisibility` (`self.NamePlate`) false false)))

(event `self.Interact`
  (bind _successfullyadded (`/Game/Blueprints/Libraries/BPFL_Inventory.AddItem` (`self.Information`) (`.Quantity_25_CB32A13742F8037488A8D990BE188642` (break `/Game/Blueprints/Structs/ST_Item` (`self.Information`)))))
  (if _successfullyadded
    (`/Game/Blueprints/Hero/Inventory/BPC_Inventory.AddSTItem` (`self.GetComponentByClass` (`self.HeroRef`) "/Game/Blueprints/Hero/Inventory/BPC_Inventory.BPC_Inventory_C") (`self.Information`))
    (`self.K2_DestroyActor`)))

(fn `UserConstructionScript`
  (bind (_datatable _rowname) (break `DataTableRowHandle` (`self.Item`)))
  (bind _returnvalue (`|GetDataTableRow` _datatable _rowname)
    (:`then`
      (set `self.Information` _returnvalue)
      (`PaperSpriteComponent.SetSprite` (`self.Model`) (`.Sprite_33_71686A9B4EE2480950F691906712C1D7` (break `/Game/Blueprints/Structs/ST_Item` (`self.Information`)))))))