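; BP_HeroController is the hero's controller Blueprint, which creates the player HUD and sets up the inventory.
; On BeginPlay it adds a BP_HUD widget to the viewport, stores the reference, then initializes an inventory with a fixed slot count and screen anchors.
; UpdateHealth pushes a new health value into the HUD's bar and text, treating 100 as full.
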(event `self.ReceiveBeginPlay`
  (`self.CreateHUD`))

(event `CreateHUD`
  (bind _returnvalue (`|CreateWidget` "/Game/Blueprints/Hero/UI/HUD/BP_HUD.BP_HUD_C"))
  (bind _output_get (set `self.HUD_REF` _returnvalue))
  (`UserWidget.AddToViewport` _output_get 0)
  ;[1 1 1] Initialize Inventory System
  (`/Game/Blueprints/Libraries/BPFL_Inventory.InitializeInventory` 12 (make `Anchors` (0.8 0.6) (1.0 0.9))))

(event `UpdateHealth`
  (params (NewHealth :type "Float (double-precision)"))
  (`ProgressBar.SetPercent` (`/Game/Blueprints/Hero/UI/HUD/BP_HUD.HealthBar` (`self.HUD_REF`)) (/ NewHealth 100.0))
  (`TextBlock.SetText` (`/Game/Blueprints/Hero/UI/HUD/BP_HUD.HealthText` (`self.HUD_REF`)) (`|FormatText` "+{Health}" NewHealth)))

(fn `UserConstructionScript`)