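; BP_NPC is a character Blueprint for an NPC that shows dialogue lines one at a time.
; Each Talk event increments DialogueIndex and, while it is within or equal to the Dialogue array length, writes that entry to the dialogue widget's text.
; The WB_Dialogue widget is created for the first player controller and added to the viewport only when no valid instance exists, then reused.
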(event `/Game/Blueprints/Dialogue/BPI_Dialogue.Talk`
  (`/Engine/EditorBlueprintResources/StandardMacros.IncrementInt` (`self.DialogueIndex`)
    (:`  `
      (if (<= (`self.DialogueIndex`) (`KismetArrayLibrary.Array_Length` (`self.Dialogue`)))
        (`self.DialogueUI`
          (:`then`
            _)
          (:`else`
            (bind _returnvalue (`|CreateWidget` "/Game/Blueprints/Hero/UI/Dialogue/WB_Dialogue.WB_Dialogue_C" (`GameplayStatics.GetPlayerController` 0)))
            (bind _output_get (set `self.DialogueUI` _returnvalue))
            (`UserWidget.AddToViewport` _output_get 0)))
        (`TextBlock.SetText` (`/Game/Blueprints/Hero/UI/Dialogue/WB_Dialogue.DialogueText` (`self.DialogueUI`)) (`KismetTextLibrary.Conv_StringToText` (`|GetArrayItem` (`self.Dialogue`) (`self.DialogueIndex`))))))))

(fn `UserConstructionScript`)